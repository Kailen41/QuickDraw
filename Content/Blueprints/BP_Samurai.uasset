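; BP_Samurai is a samurai Blueprint whose Paper2D sprite slides into place when play begins.
; BeginPlay caches the sprite's relative location as the resting position, then fires the SldieIn event.
; That event plays the SlideInAnim timeline at a raised play rate, lerping the sprite from SlideStartPos to the cached position without sweeping.
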(event `self.ReceiveBeginPlay`
  (set `self.SpriteDefaultPos` (`SceneComponent.RelativeLocation` (`self.PaperSprite`)))
  (`self.SldieIn`))

(event `SldieIn`
  (`TimelineComponent.SetPlayRate` (`self.SlideInAnim`) 1.5)
  (bind (_direction _alpha) (`Timeline|SlideInAnim` :!via `PlayFromStart`)
    (:`Update`
      (`SceneComponent.K2_SetRelativeLocation` (`self.PaperSprite`) (`KismetMathLibrary.VLerp` (`self.SlideStartPos`) (`self.SpriteDefaultPos`) _alpha) false false))))

(fn `UserConstructionScript`)