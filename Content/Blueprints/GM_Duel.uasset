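; GM_Duel runs the timing of a quick-draw duel round, from intro to the draw signal.
; On BeginPlay it caches the BP_Exclaimation actor in the level.
; Tick accumulates elapsed time and switches the phase from Intro to Wait once the round start time is reached.
; After a random delay within the draw bounds, it sets the Draw phase and makes the exclamation visible.
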(event `self.ReceiveBeginPlay`
  (bind _returnvalue (`GameplayStatics.GetActorOfClass` "/Game/Blueprints/BP_Exclaimation.BP_Exclaimation_C"))
  (set `self.Exclaimation_REF` _returnvalue))

(event `self.ReceiveTick`
  (params (DeltaSeconds :type "Float (single-precision)"))
  (bind _exclaimation_ref (`self.Exclaimation_REF`))
  (set `self.ElaspedTime` (+ DeltaSeconds (`self.ElaspedTime`)))
  (switch `/Game/Blueprints/Enums/E_Phase` (`self.Phase`)
    (:`NewEnumerator0`
      (if (>= (`self.ElaspedTime`) (`self.RoundStartTime`))
        (set `self.Phase` "NewEnumerator1")
        (`KismetSystemLibrary.Delay` (`KismetMathLibrary.RandomFloatInRange` (`self.MinDrawDelay`) (`self.MaxDrawDelay`)))
        (set `self.Phase` "NewEnumerator2")
        (`/Engine/EditorBlueprintResources/StandardMacros.IsValid` _exclaimation_ref
          (:`Is Valid`
            (`/Game/Blueprints/BP_Exclaimation.f_SetVisibility` _exclaimation_ref true)))))))

(fn `UserConstructionScript`)